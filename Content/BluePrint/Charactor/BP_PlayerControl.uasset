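; Player controller that routes movement, look, free-look, jump, crouch and prone input to BP_Player.
; Pose inputs resolve the resulting pose and transition time from data tables, pausing movement during timed transitions.
; Per-pose DataTable rows set pitch limits that gate look input, with a timeline easing out-of-range pitch to the nearest limit.
; Camera height also comes from a pose-keyed table, with a moving crouch variant, and is blended on the spring arm by timeline.
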(event Custom|SetEnableMove
  (Variables|Default|SetbIsEnableMove true))

(event EventBeginPlay
  ;[0.15 0.15 0.15 0.5] Save
  (bind _asbp_player (Utilities|Casting|CastToBP_Player (Game|Player|GetPlayerPawn 0)))
  (Variables|Default|SetBP%20Player _asbp_player)
  (CallFunction|UpdatePitchLlimits "NewEnumerator0")
  (EventDispatchers|BindEventtoCallCameraSet (Variables|Default|GetBP%20Player) (EventDispatchers|CreateEvent :!event UpDateCameraType)))

(event Input|ActionEvents|InputActionFreeLook
  (params (Key :type Key%20Structure :default "None"))
  (bind _bp_player (Variables|Default|GetBP%20Player))
  ;[0.15 0.15 0.15 0.5] FreeLook
  (:Pressed
    (Default|FreeLook _bp_player true))
  (:Released
    (Default|FreeLook _bp_player false)))

(event Input|ActionEvents|InputActionCrowch
  (params (Key :type Key%20Structure :default "None"))
  (bind _bp_player (Variables|Default|GetBP%20Player))
  (bind _currentposestate (Variables|/Game/BluePrint/Charactor/BP_Player.BP_Player_C|GetCurrentPoseState _bp_player))
  (bind _bisweaponequipped (Variables|/Game/BluePrint/Charactor/BP_Player.BP_Player_C|GetbIsWeaponEquipped _bp_player))
  (bind (_transitiontime _topose) (CallFunction|OnTransitionTimer _bisweaponequipped "NewEnumerator1" _currentposestate))
  (:Pressed
    (CallFunction|UpdatePose _topose _transitiontime)
    (CallFunction|UpdatePitchLlimits (Variables|/Game/BluePrint/Charactor/BP_Player.BP_Player_C|GetCurrentPoseState (Variables|Default|GetBP%20Player)))
    (CallFunction|UpDateCameraType false)))

(event Input|ActionEvents|InputActionProne
  (params (Key :type Key%20Structure :default "None"))
  (bind _bp_player (Variables|Default|GetBP%20Player))
  (bind _currentposestate (Variables|/Game/BluePrint/Charactor/BP_Player.BP_Player_C|GetCurrentPoseState _bp_player))
  (bind _bisweaponequipped (Variables|/Game/BluePrint/Charactor/BP_Player.BP_Player_C|GetbIsWeaponEquipped _bp_player))
  (bind (_transitiontime _topose) (CallFunction|OnTransitionTimer _bisweaponequipped "NewEnumerator2" _currentposestate))
  (:Pressed
    (CallFunction|UpdatePose _topose _transitiontime)
    (CallFunction|UpdatePitchLlimits (Variables|/Game/BluePrint/Charactor/BP_Player.BP_Player_C|GetCurrentPoseState (Variables|Default|GetBP%20Player)))
    (CallFunction|UpDateCameraType false)))

(event Input|ActionEvents|InputActionJump
  (params (Key :type Key%20Structure :default "None"))
  (bind _bp_player (Variables|Default|GetBP%20Player))
  (bind _currentposestate (Variables|/Game/BluePrint/Charactor/BP_Player.BP_Player_C|GetCurrentPoseState _bp_player))
  (bind _bisweaponequipped (Variables|/Game/BluePrint/Charactor/BP_Player.BP_Player_C|GetbIsWeaponEquipped _bp_player))
  (bind (_transitiontime _topose) (CallFunction|OnTransitionTimer _bisweaponequipped "NewEnumerator0" _currentposestate))
  (:Pressed
    (if (Utilities|Enum|Equal(Enum) _currentposestate "NewEnumerator0")
      (Character|Jump (Variables|Default|GetBP%20Player))
      (else
        (CallFunction|UpdatePose _topose _transitiontime)
        (CallFunction|UpdatePitchLlimits _topose)
        (CallFunction|UpDateCameraType false)))))

(event Input|AxisEvents|InputAxisTurn
  (params (AxisValue :type Float%20%28single-precision%29))
  ;[0.15 0.15 0.15 0.5] MouseInput
  (if (CallFunction|LimitPitchAngle AxisValue)
    (Default|InputTurn (Variables|Default|GetBP%20Player) AxisValue)))

(event Input|AxisEvents|InputAxisLookUp
  (params (AxisValue :type Float%20%28single-precision%29))
  ;[0.15 0.15 0.15 0.5] MouseInput
  (if (CallFunction|LimitPitchAngle AxisValue)
    (Default|InputLookUp (Variables|Default|GetBP%20Player) AxisValue)))

(event Input|AxisEvents|InputAxisMoveForward
  (params (AxisValue :type Float%20%28single-precision%29))
  ;[0.15 0.15 0.15 0.5] KeyboardInput
  (if (Variables|Default|GetbIsEnableMove)
    (Default|Move (Variables|Default|GetBP%20Player) true AxisValue)))

(event Input|AxisEvents|InputAxisMoveRight
  (params (AxisValue :type Float%20%28single-precision%29))
  ;[0.15 0.15 0.15 0.5] KeyboardInput
  (if (Variables|Default|GetbIsEnableMove)
    (Default|Move (Variables|Default|GetBP%20Player) false AxisValue)))

(event Custom|SetPitchTimeline
  (params (NewParam :type Rotator) (NewParam2 :type Rotator))
  (bind _newtrack_0 (Timeline|TL_PITCH PlayFromStart)
    (:Update
      (Pawn|SetControlRotation (Math|Rotator|Lerp(Rotator) NewParam2 NewParam _newtrack_0)))))

(event Custom|CameraMove
  (params (height :type Float%20%28double-precision%29) (StarkHeight :type Float%20%28double-precision%29))
  (bind _bp_player (Variables|Default|GetBP%20Player))
  (bind _springarm (Variables|/Game/BluePrint/Charactor/BP_Player.BP_Player_C|GetSpringArm _bp_player))
  (bind _newtrack_0 (Timeline|Tl_CAMERA PlayFromStart)
    (:Update
      (Variables|/Script/Engine.SpringArmComponent|SetSocketOffset _springarm (Math|Vector|MakeVector (.x (Variables|/Script/Engine.SpringArmComponent|GetSocketOffset _springarm)) (.y (Variables|/Script/Engine.SpringArmComponent|GetSocketOffset _springarm)) (Math|Float|Lerp StarkHeight height _newtrack_0))))))

(fn ConstructionScript)

(fn TryGetPoseTransition
  (params (TargetPose :type E_PoseState%20Enum :default "NewEnumerator0") (FromPose :type E_PoseState%20Enum :default "NewEnumerator0"))
  (bind _returnvalue (Utilities|String|EnumtoString TargetPose))
  (bind _returnvalue_2 (Utilities|String|EnumtoString FromPose))
  (Development|PrintString (Utilities|String|ToString(Text) (Utilities|Text|FormatText "{1} :: {2}" _returnvalue _returnvalue_2)))
  (bind _returnvalue_3 (Utilities|GetDataTableRow "/Game/BluePrint/Datas/DataTable/DT_PoseTransitions.DT_PoseTransitions" (Utilities|String|StringToName (Utilities|String|Append _returnvalue "_" _returnvalue_2)))
    (:then
      (return (.topose _returnvalue_3)))))

(fn OnTransitionTimer
  (params (bIsWeaponEquipped :type Boolean) (TargetPose :type E_PoseState%20Enum :default "NewEnumerator0") (FromPose :type E_PoseState%20Enum :default "NewEnumerator0"))
  (LocalVariables|SetReturn (CallFunction|TryGetPoseTransition TargetPose FromPose))
  (bind _returnvalue (Utilities|GetDataTableRow "/Game/BluePrint/Datas/DataTable/DT_ProneTime.DT_ProneTime" (Utilities|String|StringToName (Utilities|String|Append (Utilities|String|ToString(Boolean) bIsWeaponEquipped) "_" (Utilities|String|EnumtoString FromPose) "_" (Utilities|String|EnumtoString (LocalVariables|GetReturn)))))
    (:then
      _)
    (:RowNotFound
      _))
  (return (.sec _returnvalue) (LocalVariables|GetReturn)))

(fn UpdatePose
  (params (ToPose :type E_PoseState%20Enum :default "NewEnumerator0") (WaitTIme :type Float%20%28double-precision%29))
  (if (!= WaitTIme 0.0)
    (Variables|Default|SetbIsEnableMove false)
    (Utilities|Time|SetTimerbyEvent (EventDispatchers|CreateEvent :!event Custom|SetEnableMove) WaitTIme))
  (Default|UpdatePose (Variables|Default|GetBP%20Player) ToPose))

(fn UpdatePitchLlimits
  (params (ToPose :type E_PoseState%20Enum :default "NewEnumerator0"))
  (bind _returnvalue (Pawn|GetControlRotation :!class /Script/Engine.Controller))
  (bind _returnvalue_2 (Pawn|GetControlRotation :!class /Script/Engine.Controller))
  (bind _returnvalue_3 (Pawn|GetControlRotation :!class /Script/Engine.Controller))
  (Utilities|FlowControl|Sequence
    (:then_0
      (bind _returnvalue_4 (Utilities|GetDataTableRow "/Game/BluePrint/Datas/DataTable/DT_PitchLimit.DT_PitchLimit" (Utilities|String|StringToName (Utilities|String|EnumtoString ToPose)))
        (:then
          (Variables|Default|SetCachedBottomLimit (.bottomlimit _returnvalue_4))
          (Variables|Default|SetCachedTopLimit (.toplimit _returnvalue_4)))))
    (:then_1
      (if (not (or (> (.pitch _returnvalue_3) (Variables|Default|GetCachedBottomLimit)) (< (.pitch _returnvalue_3) (Variables|Default|GetCachedTopLimit))))
        (if (< (Math|Float|Absolute(Float) (- (.pitch _returnvalue_3) (Variables|Default|GetCachedTopLimit))) (Math|Float|Absolute(Float) (- (.pitch _returnvalue_3) (Variables|Default|GetCachedBottomLimit))))
          (CallFunction|SetPitchTimeline (Math|Rotator|MakeRotator (.roll _returnvalue_2) (Variables|Default|GetCachedTopLimit) (.yaw _returnvalue_2)) _returnvalue)
          (else
            (CallFunction|SetPitchTimeline (Math|Rotator|MakeRotator (.roll _returnvalue_2) (Variables|Default|GetCachedBottomLimit) (.yaw _returnvalue_2)) _returnvalue)))))))

(fn LimitPitchAngle
  (params (Axix :type Float%20%28double-precision%29))
  (bind _returnvalue (Pawn|GetControlRotation :!class /Script/Engine.Controller))
  (bind _returnvalue_2 (Class|PlayerController|GetDeprecatedInputPitchScale))
  (bind _returnvalue_3 (* Axix _returnvalue_2))
  (bind _returnvalue_4 (+ (.pitch _returnvalue) _returnvalue_3))
  (return (or (< (Variables|Default|GetCachedBottomLimit) _returnvalue_4) (> (Variables|Default|GetCachedTopLimit) _returnvalue_4))))

(fn UpDateCameraType
  (params (bIsMovingNow :type Boolean))
  (bind _bp_player (Variables|Default|GetBP%20Player))
  (bind _currentposestate (Variables|/Game/BluePrint/Charactor/BP_Player.BP_Player_C|GetCurrentPoseState _bp_player))
  (Utilities|FlowControl|Sequence
    (:then_0
      (LocalVariables|SetCurrentPose (Utilities|String|EnumtoString _currentposestate))
      (LocalVariables|SetRowName (LocalVariables|GetCurrentPose))
      (if (not (Utilities|Enum|NotEqual(Enum) _currentposestate "NewEnumerator1"))
        (if bIsMovingNow
          (LocalVariables|SetRowName (Utilities|String|Append (LocalVariables|GetCurrentPose) "_" (Utilities|String|ToString(Boolean) (Variables|/Game/BluePrint/Charactor/BP_Player.BP_Player_C|GetbIsWeaponEquipped (Variables|Default|GetBP%20Player))) "_Move")))))
    (:then_1
      (bind _returnvalue (Utilities|GetDataTableRow "/Game/BluePrint/Datas/DataTable/DT_CameraHigh.DT_CameraHigh" (Utilities|String|StringToName (LocalVariables|GetRowName)))
        (:then
          (CallFunction|CameraMove (.high _returnvalue) (.z (Variables|/Script/Engine.SpringArmComponent|GetSocketOffset (Variables|/Game/BluePrint/Charactor/BP_Player.BP_Player_C|GetSpringArm (Variables|Default|GetBP%20Player))))))))))