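; Player character Blueprint providing movement, mouse-look, free-look and pose state functions.
; FreeLook saves the control rotation and releases controller yaw, then on release re-enables it while a timeline lerps the view back.
; Move takes its direction from a yaw helper fed the free-look flag, and Tick signals camera changes when movement starts or stops.
; Speed-ramp logic in Move is disconnected, and InputLookUp prints pitch for debugging.
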(event EventBeginPlay)

(event EventTick
  (params (DeltaSeconds :type Float%20%28single-precision%29))
  (bind _returnvalue (Transformation|GetVelocity))
  (bind _returnvalue_2 (Math|Vector|VectorLengthSquared _returnvalue))
  (bind _returnvalue_3 (> _returnvalue_2 0.0))
  (if (!= (Variables|Default|GetbIsMoving) _returnvalue_3)
    (bind _output_get (Variables|Default|SetbIsMoving _returnvalue_3))
    (Default|CallCallCameraSet _output_get)))

(event Custom|OnFreeLookEnded
  (bind _newtrack_0 (Timeline|Timeline PlayFromStart)
    (:Update
      (Pawn|SetControlRotation (Pawn|GetController) (Math|Rotator|Lerp(Rotator) (Variables|FreeLook|GetFreeLookEndRatation_0) (Variables|FreeLook|GetFreeLookStartRatation) _newtrack_0 true)))
    (:Finished
      (Variables|Default|SetbUseControllerRotationYaw true))))

(fn ConstructionScript)

(fn InputLookUp
  (params (YAxix :type Float%20%28double-precision%29))
  (Pawn|Input|AddControllerPitchInput YAxix)
  (Development|PrintString (Utilities|String|ToString(Float) (.pitch (Pawn|GetControlRotation :!class /Script/Engine.Pawn))) true true "(R=0.000000,G=0.660000,B=1.000000,A=1.000000)" 0.0))

(fn Move
  (params (BisForward :type Boolean) (Axisvalue :type Float%20%28double-precision%29))
  (bind _self self)
  (bind _freelookon (Variables|FreeLook|GetFreeLookOn))
  (bind _yawrotator (CallFunction|GetYawRotation _self _freelookon))
  (if BisForward
    (Pawn|Input|AddMovementInput (Math|Vector|GetForwardVector _yawrotator) Axisvalue false)
    (else
      (Pawn|Input|AddMovementInput (Math|Vector|GetRightVector _yawrotator) Axisvalue false))))

(fn InputTurn
  (params (XAxis :type Float%20%28double-precision%29))
  (Pawn|Input|AddControllerYawInput XAxis))

(fn FreeLook
  (params (Pressed :type Boolean))
  (bind _returnvalue (Pawn|GetControlRotation :!class /Script/Engine.Pawn))
  (if Pressed
    (Variables|FreeLook|SetFreeLookStartRatation _returnvalue)
    (Variables|Default|SetbUseControllerRotationYaw false)
    (Variables|FreeLook|SetFreeLookOn true)
    (else
      (Variables|FreeLook|SetFreeLookEndRatation_0 _returnvalue)
      (Variables|Default|SetbUseControllerRotationYaw true)
      (CallFunction|OnFreeLookEnded)
      (Variables|FreeLook|SetFreeLookOn false))))

(fn UpdatePose
  (params (NewState :type E_PoseState%20Enum :default "NewEnumerator0"))
  (Variables|Pose|SetCurrentPoseState NewState))